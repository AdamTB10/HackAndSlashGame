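; BP_MainMenu is an actor Blueprint that displays the main menu of the hack-and-slash game when play begins.
; BeginPlay reuses the stored WBP_MainMenu widget if it is valid, otherwise creates it and adds it to the viewport.
; It switches the first player controller to UI-only input, then gives the Play button focus after a short delay.
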(event `self.ReceiveBeginPlay`
  (bind _mainmenu (`self.MainMenu`))
  (bind _mainmenu_2 (`self.MainMenu`)
    (:`then`
      (`Widget.SetVisibility` _mainmenu_2 "Visible"))
    (:`else`
      (bind _returnvalue (`|CreateWidget` "/Game/HackAndSlashGame/UI/Menus/WBP_MainMenu.WBP_MainMenu_C"))
      (bind _output_get (set `self.MainMenu` _returnvalue))
      (`UserWidget.AddToViewport` _output_get 0)))
  (`WidgetBlueprintLibrary.SetInputMode_UIOnlyEx` (`GameplayStatics.GetPlayerController` 0) _mainmenu)
  (`KismetSystemLibrary.Delay` 0.2)
  (`Widget.SetFocus` (`/Game/HackAndSlashGame/UI/Menus/WBP_MainMenu.PlayButton` _mainmenu)))

(fn `UserConstructionScript`)