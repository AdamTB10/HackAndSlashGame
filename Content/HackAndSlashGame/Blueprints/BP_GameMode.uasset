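; Game mode for a hack-and-slash game that runs enemy waves, starts the music and ends in a win screen.
; Each WaveSystemDataTable row defines up to five enemy types and counts, which SpawnSystem spawns at random TargetPoints gathered on BeginPlay.
; EnemyWasKilled counts kills against the wave total, then advances the wave and updates the player HUD.
; After the last wave, EndGame shows WBP_WinMenu with UI-only input and pauses the game.
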(event `self.ReceiveBeginPlay`
  (bind _outactors (`GameplayStatics.GetAllActorsOfClass` "/Script/Engine.TargetPoint"))
  (bind _output_get (set `self.spawnPoints` _outactors))
  (bind _result (`/Engine/EditorBlueprintResources/StandardMacros.DecrementInt` (`KismetArrayLibrary.Array_Length` _output_get))
    (:`  `
      (set `self.numOfSpawnPoints` _result)
      (bind _outrownames (`DataTableFunctionLibrary.GetDataTableRowNames` (`self.waveSystemDataTable`)))
      (set `self.maxWaves` (`KismetArrayLibrary.Array_Length` _outrownames))
      (`self.spawnWave`)
      (bind _asbp_player (cast `/Game/HackAndSlashGame/Blueprints/Player/BP_Player` (`GameplayStatics.GetPlayerPawn` 0)))
      (bind _playerhud (`/Game/HackAndSlashGame/Blueprints/Player/BP_Player.PlayerHUD` _asbp_player))
      (`/Engine/EditorBlueprintResources/StandardMacros.IsValid` _playerhud
        (:`Is Valid`
          (`/Game/HackAndSlashGame/UI/HUD/WBP_PlayerHUD.updateCurrentWave` _playerhud (`self.currentWave`)))
        (:`Is Not Valid`
          _))
      (`GameplayStatics.PlaySound2D` "/Game/HackAndSlashGame/Audio/BGM/SC_Royal_Captial_Loop.SC_Royal_Captial_Loop" 0.5 1.0 0.0 null null))))

(event `spawnWave`
  (bind _outrownames (`DataTableFunctionLibrary.GetDataTableRowNames` (`self.waveSystemDataTable`)))
  (bind _returnvalue (`|GetDataTableRow` (`self.waveSystemDataTable`) (`|GetArrayItem` _outrownames (`self.currentWave`)))
    (:`then`
      (bind (_enemy1 _numofenemy1 _enemy2 _numofenemy2 _enemy3 _numofenemy3 _enemy4 _numofenemy4 _enemy5 _numofenemy5) (break `/Game/HackAndSlashGame/Blueprints/Datatable/STC_EnemyWaves` _returnvalue))
      (set `self.killNeeded` (+ _numofenemy1 _numofenemy2 _numofenemy3 _numofenemy4 _numofenemy5))
      (bind (_enemy1_2 _numofenemy1_2 _enemy2_2 _numofenemy2_2 _enemy3_2 _numofenemy3_2 _enemy4_2 _numofenemy4_2 _enemy5_2 _numofenemy5_2) (break `/Game/HackAndSlashGame/Blueprints/Datatable/STC_EnemyWaves` _returnvalue))
      (`self.SpawnSystem` _enemy1_2 _numofenemy1_2)
      (`self.SpawnSystem` _enemy2_2 _numofenemy2_2)
      (`self.SpawnSystem` _enemy3_2 _numofenemy3_2)
      (`self.SpawnSystem` _enemy4_2 _numofenemy4_2)
      (`self.SpawnSystem` _enemy5_2 _numofenemy5_2))))

(event `enemyWasKilled`
  (bind _result (`/Engine/EditorBlueprintResources/StandardMacros.IncrementInt` (`self.currentKills`))
    (:`  `
      (if (>= _result (`self.killNeeded`))
        (set `self.killNeeded` 0)
        (set `self.currentKills` 0)
        (bind _result_2 (`/Engine/EditorBlueprintResources/StandardMacros.IncrementInt` (`self.currentWave`))
          (:`  `
            (if (< _result_2 (`self.maxWaves`))
              (`self.spawnWave`)
              (bind _asbp_player (cast `/Game/HackAndSlashGame/Blueprints/Player/BP_Player` (`GameplayStatics.GetPlayerPawn` 0)))
              (`/Game/HackAndSlashGame/UI/HUD/WBP_PlayerHUD.updateCurrentWave` (`/Game/HackAndSlashGame/Blueprints/Player/BP_Player.PlayerHUD` _asbp_player) (`self.currentWave`))
              (else
                (`self.endGame`)))))))))

(event `endGame`
  (bind _winmenu (`self.winMenu`))
  (bind _winmenu_2 (`self.winMenu`)
    (:`then`
      (`Widget.SetVisibility` _winmenu_2 "Visible"))
    (:`else`
      (bind _returnvalue (`|CreateWidget` "/Game/HackAndSlashGame/UI/Menus/WBP_WinMenu.WBP_WinMenu_C"))
      (bind _output_get (set `self.winMenu` _returnvalue))
      (`UserWidget.AddToViewport` _output_get 1)))
  (`WidgetBlueprintLibrary.SetInputMode_UIOnlyEx` (`GameplayStatics.GetPlayerController` 0) _winmenu)
  (`KismetSystemLibrary.Delay` 0.2)
  (`Widget.SetFocus` (`/Game/HackAndSlashGame/UI/Menus/WBP_WinMenu.ResumeButton` _winmenu))
  (`GameplayStatics.SetGamePaused` true))

(fn `SpawnSystem`
  (params (EnemyToSpawn :type "Actor Class Reference") (Num :type Integer))
  (bind _returnvalue_location (`KismetMathLibrary.BreakTransform` (`self.GetTransform` (`|GetArrayItem` (`self.spawnPoints`) (`KismetMathLibrary.RandomIntegerInRange` 0 (`self.numOfSpawnPoints`))))))
  (if (> Num 0)
    (bind _result (`/Engine/EditorBlueprintResources/StandardMacros.DecrementInt` Num)
      (:`  `
        (for _ (range (+ _result 1))
          (`|SpawnActorFromClass` EnemyToSpawn (`KismetMathLibrary.MakeTransform` _returnvalue_location) "AdjustIfPossibleButAlwaysSpawn" "MultiplyWithRoot" null null))))))

(fn `UserConstructionScript`)