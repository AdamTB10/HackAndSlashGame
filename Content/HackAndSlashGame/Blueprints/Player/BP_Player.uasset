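; Player character for a hack-and-slash game, handling Enhanced Input movement, look, jump with a double-jump montage, lock-on and sword attacks.
; Lock-on caches the nearest BP_BaseEnemy, eases control rotation toward it while held and keeps a reticle above it until release.
; Attacks step through two alternating four-hit montage combos, with notifies reopening input, resetting the combo and toggling the sword's hit collision.
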(event `self.ReceiveBeginPlay`
  (`EnhancedInputSubsystemInterface.AddMappingContext` (pcsubsystem `EnhancedInputLocalPlayerSubsystem` (`GameplayStatics.GetPlayerController` 0)) "/Game/HackAndSlashGame/Inputs/IMC_PlayerControls.IMC_PlayerControls" 0 (struct))
  (`PrimitiveComponent.SetCollisionEnabled` (`self.HeroSword`) "NoCollision"))

(event `EnhancedInput|/Game/HackAndSlashGame/Inputs/IA_Move`
  (params (ActionValue :type "Vector2D Structure") (ElapsedSeconds :type "Float (double-precision)") (TriggeredSeconds :type "Float (double-precision)") (InputAction :type "InputAction Object Reference" :default "/Game/HackAndSlashGame/Inputs/IA_Move.IA_Move"))
  (:`Triggered`
    (`self.AddMovementInput` (`self.GetActorForwardVector`) ActionValue_X)
    (`self.AddMovementInput` (`self.GetActorRightVector`) ActionValue_Y))
  (:`Started`
    (set `self.bUseControllerRotationYaw` true))
  (:`Completed`
    (set `self.bUseControllerRotationYaw` false)))

(event `EnhancedInput|/Game/HackAndSlashGame/Inputs/IA_Lockon`
  (params (ActionValue :type Boolean) (ElapsedSeconds :type "Float (double-precision)") (TriggeredSeconds :type "Float (double-precision)") (InputAction :type "InputAction Object Reference" :default "/Game/HackAndSlashGame/Inputs/IA_Lockon.IA_Lockon"))
  (bind _returnvalue (`GameplayStatics.GetPlayerController` 0))
  (:`Triggered`
    (`self.nearestEnemy`
      (:`then`
        (`Controller.SetControlRotation` _returnvalue (`KismetMathLibrary.RLerp` (`Controller.GetControlRotation` _returnvalue) (`KismetMathLibrary.FindLookAtRotation` (`self.K2_GetActorLocation`) (`self.K2_GetActorLocation` (`self.nearestEnemy`))) 0.1 true))
        (`self.lockonReticle`
          (:`then`
            (bind _returnvalue_2 (`GameplayStatics.GetActorOfClass` "/Game/HackAndSlashGame/Blueprints/Player/BP_LockonReticle.BP_LockonReticle_C"))
            (`self.K2_SetActorLocation` _returnvalue_2 (+ (`self.K2_GetActorLocation` (`self.nearestEnemy`)) (0.0 0.0 40.0)) false false))
          (:`else`
            (bind _returnvalue_3 (`|SpawnActorFromClass` "/Game/HackAndSlashGame/Blueprints/Player/BP_LockonReticle.BP_LockonReticle_C" (`KismetMathLibrary.MakeTransform` (+ (`self.K2_GetActorLocation` (`self.nearestEnemy`)) (0.0 0.0 40.0))) "Undefined" "MultiplyWithRoot" null null))
            (set `self.lockonReticle` _returnvalue_3))))
      (:`else`
        (bind _outactors (`GameplayStatics.GetAllActorsOfClass` "/Game/HackAndSlashGame/Blueprints/Enemies/BP_BaseEnemy.BP_BaseEnemy_C" :!label _label))
        (set `self.nearestEnemy` (`.ReturnValue` (`GameplayStatics.FindNearestActor` (`self.K2_GetActorLocation`) _outactors))))))
  (:`Started`
    (goto _label))
  (:`Completed`
    (`self.K2_DestroyActor` (`self.lockonReticle`))))

(event `EnhancedInput|/Game/HackAndSlashGame/Inputs/IA_Look`
  (params (ActionValue :type "Vector2D Structure") (ElapsedSeconds :type "Float (double-precision)") (TriggeredSeconds :type "Float (double-precision)") (InputAction :type "InputAction Object Reference" :default "/Game/HackAndSlashGame/Inputs/IA_Look.IA_Look"))
  (:`Triggered`
    (`self.AddControllerYawInput` ActionValue_X)
    (`self.AddControllerPitchInput` (* ActionValue_Y -1.0))))

(event `EnhancedInput|/Game/HackAndSlashGame/Inputs/IA_Jump`
  (params (ActionValue :type Boolean) (ElapsedSeconds :type "Float (double-precision)") (TriggeredSeconds :type "Float (double-precision)") (InputAction :type "InputAction Object Reference" :default "/Game/HackAndSlashGame/Inputs/IA_Jump.IA_Jump"))
  (:`Started`
    (`self.Jump`)
    (`|PlayMontage` (`self.Mesh`) (select `int` (`self.JumpCurrentCount`) :`0` null :`1` "/Game/HackAndSlashGame/Animations/Characters/Jump/DoubleJump/AM_DoubleJump.AM_DoubleJump" :!type "AnimMontage Object Reference"))))

(event `EnhancedInput|/Game/HackAndSlashGame/Inputs/IA_Attack`
  (params (ActionValue :type Boolean) (ElapsedSeconds :type "Float (double-precision)") (TriggeredSeconds :type "Float (double-precision)") (InputAction :type "InputAction Object Reference" :default "/Game/HackAndSlashGame/Inputs/IA_Attack.IA_Attack"))
  (:`Started`
    (if (`self.canAttack`)
      (set `self.canAttack` false)
      (switch `int` (`self.ComboSelecter`)
        (:`0`
          (bind _notifyname (`|PlayMontage` (`self.Mesh`) (select `int` (`self.ComboAttackIndex`) :`0` "/Game/HackAndSlashGame/Animations/Characters/Attack/ComboAttack01/AM_ComboAttack01_01.AM_ComboAttack01_01" :`1` "/Game/HackAndSlashGame/Animations/Characters/Attack/ComboAttack01/AM_ComboAttack01_02.AM_ComboAttack01_02" :`2` "/Game/HackAndSlashGame/Animations/Characters/Attack/ComboAttack01/AM_ComboAttack01_03.AM_ComboAttack01_03" :`3` "/Game/HackAndSlashGame/Animations/Characters/Attack/ComboAttack01/AM_ComboAttack01_04.AM_ComboAttack01_04" :!type "AnimMontage Object Reference"))
            (:`then`
              (bind _result (`/Engine/EditorBlueprintResources/StandardMacros.IncrementInt` (`self.ComboAttackIndex`) :!label _label_2)
                (:`  `
                  (if (>= _result 4)
                    (set `self.ComboAttackIndex` 0)
                    (set `self.ComboSelecter` (`KismetMathLibrary.SelectInt` 1 0 (== (`self.ComboSelecter`) 0)))))))
            (:`OnNotifyBegin`
              (switch `name` _notifyname
                (:`canAttack`
                  (set `self.canAttack` true))
                (:`resetCombo`
                  (set `self.ComboAttackIndex` 0)
                  (set `self.canAttack` true))
                (:`hitboxActive`
                  (`PrimitiveComponent.SetCollisionEnabled` (`self.HeroSword`) "QueryOnly"))))
            (:`OnNotifyEnd`
              (`PrimitiveComponent.SetCollisionEnabled` (`self.HeroSword`) "NoCollision"))))
        (:`1`
          (bind _notifyname_2 (`|PlayMontage` (`self.Mesh`) (select `int` (`self.ComboAttackIndex`) :`0` "/Game/HackAndSlashGame/Animations/Characters/Attack/ComboAttack02/AM_ComboAttack02_01.AM_ComboAttack02_01" :`1` "/Game/HackAndSlashGame/Animations/Characters/Attack/ComboAttack02/AM_ComboAttack02_02.AM_ComboAttack02_02" :`2` "/Game/HackAndSlashGame/Animations/Characters/Attack/ComboAttack02/AM_ComboAttack02_03.AM_ComboAttack02_03" :`3` "/Game/HackAndSlashGame/Animations/Characters/Attack/ComboAttack02/AM_ComboAttack02_04.AM_ComboAttack02_04" :!type "AnimMontage Object Reference"))
            (:`then`
              (goto _label_2))
            (:`OnNotifyBegin`
              (switch `name` _notifyname_2
                (:`canAttack`
                  (set `self.canAttack` true))
                (:`resetCombo`
                  (set `self.ComboAttackIndex` 0)
                  (set `self.canAttack` true))
                (:`hitboxActive`
                  (`PrimitiveComponent.SetCollisionEnabled` (`self.HeroSword`) "QueryOnly"))))
            (:`OnNotifyEnd`
              (`PrimitiveComponent.SetCollisionEnabled` (`self.HeroSword`) "NoCollision"))))))))

(fn `UserConstructionScript`)