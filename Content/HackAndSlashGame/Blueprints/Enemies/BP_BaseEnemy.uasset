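; Base enemy for a hack-and-slash game that tracks health, takes damage, reacts to hits and dies.
; Non-lethal hits play one of four directional montages, chosen by dot products of the damage causer's direction against the enemy's forward and right vectors.
; Montage notifies open and close an invulnerability window, while lethal damage plays a death montage and destroys the actor on blend out.
; Tick matches the HUD arrow's world rotation to the player controller's.
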(event `self.ReceiveBeginPlay`
  (set `self.currentHealth` (`self.maxHealth`)))

(event `self.ReceiveTick`
  (params (DeltaSeconds :type "Float (single-precision)"))
  (`SceneComponent.K2_SetWorldRotation` (`self.HUDArrow`) (`self.K2_GetActorRotation` (`GameplayStatics.GetPlayerController` 0)) false false))

(event `self.ReceiveAnyDamage`
  (params (Damage :type "Float (single-precision)") (DamageType :type "DamageType Object Reference") (InstigatedBy :type "Controller Object Reference") (DamageCauser :type "Actor Object Reference"))
  (bind _returnvalue (`KismetMathLibrary.Normal` (- (`self.K2_GetActorLocation`) (`self.K2_GetActorLocation` DamageCauser))))
  (bind _returnvalue_2 (`KismetMathLibrary.Dot_VectorVector` _returnvalue (`KismetMathLibrary.Normal` (`self.GetActorForwardVector`))))
  (if (`self.canBeDamaged`)
    (bind _output_get (set `self.currentHealth` (- (`self.currentHealth`) Damage)))
    (if (<= _output_get 0.0)
      (set `self.canBeDamaged` false)
      (`|PlayMontage` (`self.Mesh`) "/Game/HackAndSlashGame/Animations/Sequences/Hit/Hit/AM_Death.AM_Death"
        (:`OnBlendOut`
          (`self.K2_DestroyActor`)))
      (else
        (if (> _returnvalue_2 0.5)
          (set `self.hitAnimation` "/Game/HackAndSlashGame/Animations/Sequences/Hit/Hit/AM_HitBack.AM_HitBack")
          (elif (< _returnvalue_2 -0.5)
            (set `self.hitAnimation` "/Game/HackAndSlashGame/Animations/Sequences/Hit/Hit/AM_HitForward.AM_HitForward")
            (elif (> (`KismetMathLibrary.Dot_VectorVector` _returnvalue (`KismetMathLibrary.Normal` (`self.GetActorRightVector`))) 0.0)
              (set `self.hitAnimation` "/Game/HackAndSlashGame/Animations/Sequences/Hit/Hit/AM_HitRight.AM_HitRight")
              (else
                (set `self.hitAnimation` "/Game/HackAndSlashGame/Animations/Sequences/Hit/Hit/AM_HitLeft.AM_HitLeft")))))
        (`|PlayMontage` (`self.Mesh`) (`self.hitAnimation`)
          (:`OnNotifyBegin`
            (set `self.canBeDamaged` false))
          (:`OnNotifyEnd`
            (set `self.canBeDamaged` true)))))))

(fn `UserConstructionScript`)