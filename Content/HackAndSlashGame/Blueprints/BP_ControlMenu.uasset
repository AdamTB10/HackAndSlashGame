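; BP_ControlMenu is a Blueprint that displays the controls screen, WBP_Controls, when it begins play.
; It makes an existing ControlMenu widget visible, or creates one and adds it to the viewport if none is valid.
; It then switches the player controller to UI-only input and, after a short delay, focuses the widget's main menu button.
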(event `self.ReceiveBeginPlay`
  (bind _controlmenu (`self.controlMenu`))
  (bind _controlmenu_2 (`self.controlMenu`)
    (:`then`
      (`Widget.SetVisibility` _controlmenu_2 "Visible"))
    (:`else`
      (bind _returnvalue (`|CreateWidget` "/Game/HackAndSlashGame/UI/Menus/WBP_Controls.WBP_Controls_C"))
      (bind _output_get (set `self.controlMenu` _returnvalue))
      (`UserWidget.AddToViewport` _output_get 0)))
  (`WidgetBlueprintLibrary.SetInputMode_UIOnlyEx` (`GameplayStatics.GetPlayerController` 0) _controlmenu)
  (`KismetSystemLibrary.Delay` 0.2)
  (`Widget.SetFocus` (`/Game/HackAndSlashGame/UI/Menus/WBP_Controls.MainMenuButton` _controlmenu)))

(fn `UserConstructionScript`)